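; BP_gamemodetest is a test game mode, judging by its name, that runs a countdown timer and closes the game when time runs out.
; While GameRunning is set, Tick subtracts delta time from GameTime, then at zero clears the flag, clamps the time and calls QuitGame.
; Score logic exists only as disconnected leftover nodes, and BeginPlay and the construction script are empty.
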(event `self.ReceiveBeginPlay`)

(event `self.ReceiveTick`
  (params (DeltaSeconds :type "Float (single-precision)"))
  (if (`self.game running`)
    (bind _output_get (set `self.GameTime` (- (`self.GameTime`) DeltaSeconds)))
    (if (<= _output_get 0.0)
      (set `self.game running` false)
      (set `self.GameTime` 0.0)
      (`KismetSystemLibrary.QuitGame` null "Quit"))))

(fn `UserConstructionScript`)